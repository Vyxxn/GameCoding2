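; BP_Turret is an AI turret that fires bullets at a sensed enemy.
; A sight event sets or clears EnemyTarget and starts Attack, which spawns BP_Bullet at BulletSpawnPoint and re-calls itself after a delay set by RoundsPerMinute.
; Tick rotates Pivot along the target's velocity, offset from the turret's own location; the target's position is unused, so it does not aim at the enemy itself.
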(event `self.ReceiveTick`
  (params (DeltaSeconds :type "Float (single-precision)"))
  (bind _returnvalue (`SceneComponent.K2_GetComponentLocation` (`self.DefaultSceneRoot`)))
  (`self.EnemyTarget`
    (:`then`
      (`SceneComponent.K2_SetWorldRotation` (`self.Pivot`) (`KismetMathLibrary.FindLookAtRotation` _returnvalue (+ _returnvalue (* (`self.GetVelocity` (`self.EnemyTarget`)) 0.2))) false false))
    (:`else`)))

(event `Attack`
  (`self.EnemyTarget`
    (:`then`
      (`|SpawnActorFromClass` "/Game/Blueprints/BP_Bullet.BP_Bullet_C" (`SceneComponent.K2_GetComponentToWorld` (`self.BulletSpawnPoint`)) "Undefined" "MultiplyWithRoot" null null)
      (`KismetSystemLibrary.Delay` (/ 60.0 (`self.RoundsPerMinute`)))
      (`self.Attack`))
    (:`else`)))

(event `Handle Sight_1`
  (params (Target :type "Actor Object Reference") (`Successfully Sensed` :type Boolean) (Location :type "Vector Structure"))
  (if `Successfully Sensed`
    (set `self.EnemyTarget` Target)
    (`self.Attack`)
    (else
      (set `self.EnemyTarget` null))))

(fn `UserConstructionScript`)