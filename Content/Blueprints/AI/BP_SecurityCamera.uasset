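; BP_SecurityCamera is an AI security camera that reacts to sight of the player with Looking, Investigating and Alert states, each shown by a material swap.
; HandleSight records visibility and starts investigating from Looking; a one-second delay then escalates to Alert or resets.
; Alert re-checks each second, dropping to Investigating when sight is lost.
; Its BP_DumDum loop is empty, and the GoToSecPoint call is unconnected.
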(event `HandleSight`
  (params (`Successfully Sensed` :type Boolean) (Target :type "Actor Object Reference"))
  (set `self.CurrentlySeePlayer` `Successfully Sensed`)
  (switch `/Game/Blueprints/AI/E_CamState` (`self.CameraState`) ; what state are we in
    (:`NewEnumerator0`
      (`self.Investigating` (`self.CurrentlySeePlayer`)))))

(event `Investigating`
  (params (Sensed :type Boolean))
  (set `self.CameraState` "NewEnumerator1")
  (`PrimitiveComponent.SetMaterial` (`self.StaticMesh`) 0 "/Game/Fantastic_Dungeon_Pack/materials/MI_CLR_yellow_E.MI_CLR_yellow_E") ; Change color to yellow
  (`KismetSystemLibrary.Delay` 1.0)
  (if (`self.CurrentlySeePlayer`)
    (`self.Alert`)
    (else
      (`self.Looking`))))

(event `Alert`
  (if (`self.CurrentlySeePlayer`)
    (set `self.CameraState` "NewEnumerator2")
    (`PrimitiveComponent.SetMaterial` (`self.StaticMesh`) 0 "/AnimationSharing/AnimSharingRed.AnimSharingRed")
    (bind _outactors (`GameplayStatics.GetAllActorsOfClass` "/Game/Blueprints/AI/BP_DumDum.BP_DumDum_C"))
    (for _ _outactors
      _)
    (`KismetSystemLibrary.Delay` 1.0)
    (`self.Alert`)
    (else
      (`self.Investigating` false))))

(event `Looking`
  (set `self.CameraState` "NewEnumerator0")
  (`PrimitiveComponent.SetMaterial` (`self.StaticMesh`) 0 "/Engine/MapTemplates/Sky/M_BlackBackground.M_BlackBackground"))

(fn `UserConstructionScript`)