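; AI controller, named for melee enemies, that turns perception of actors not tagged "AI" into StateTree events.
; Sight sets the target and sends Attacking, while hearing stores the location and sends Investigating.
; Damage records the attacker's location and sends an event without a visible tag.
; Losing sight starts a retriggerable delay before clearing the target; the security camera reference cached on possess is used only in unreached code.
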(event `self.AIPerception.OnTargetPerceptionUpdated`
  (params (Actor :type "Actor Object Reference") (Stimulus :type "AIStimulus Structure"))
  (bind (_age _expirationage _strength _stimuluslocation _receiverlocation _tag _bsuccessfullysensed) (break `AIStimulus` Stimulus))
  (if (not (`self.ActorHasTag` Actor "AI"))
    (bind _returnvalue (`AIPerceptionSystem.GetSenseClassForStimulus` Stimulus))
    (switch `string` (`KismetSystemLibrary.GetClassDisplayName` _returnvalue)
      (:`AISense_Sight`
        (`self.Handle Sight` _bsuccessfullysensed Actor))
      (:`AISense_Hearing`
        (`self.Handle Sound` _stimuluslocation))
      (:`AISense_Damage`
        (`self.Handle Damage` _stimuluslocation Actor)))))

(event `self.ReceivePossess`
  (params (PossessedPawn :type "Pawn Object Reference"))
  (bind _asbp_security_camera (cast `/Game/Blueprints/AI/BP_SecurityCamera` PossessedPawn))
  (set `self.As BP Security Camera` _asbp_security_camera))

(event `Lose Sight Delay`
  (set `self.CanSeePlayer` false)
  (`KismetSystemLibrary.RetriggerableDelay` (`self.Duration`))
  (if (not (`self.CanSeePlayer`))
    (set `self.Target Actor` null)))

(fn `Handle Damage`
  (params (`Point of Interest` :type "Vector Structure") (Attacker :type "Actor Object Reference"))
  (set `self.Point Of Interest` (`self.K2_GetActorLocation` Attacker))
  (`StateTreeComponent.SendStateTreeEvent` (`self.StateTreeAI`) (make `StateTreeEvent` (struct))))

(fn `Handle Sight`
  (params (`Successfully Sensed` :type Boolean) (Target :type "Actor Object Reference"))
  (if `Successfully Sensed`
    (set `self.CanSeePlayer` true)
    (set `self.Target Actor` Target)
    (`StateTreeComponent.SendStateTreeEvent` (`self.StateTreeAI`) (make `StateTreeEvent` :`Tag` (struct :`TagName` "AI.Event.Attacking")))
    (else
      (`self.Lose Sight Delay`))))

(fn `Handle Sound`
  (params (Location :type "Vector Structure"))
  (set `self.HeardLocation` Location)
  (`StateTreeComponent.SendStateTreeEvent` (`self.StateTreeAI`) (make `StateTreeEvent` :`Tag` (struct :`TagName` "ai.event.investigating"))))

(fn `UserConstructionScript`)