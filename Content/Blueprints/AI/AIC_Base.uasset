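; AIC_Base is an AI controller that relays sight perception to the security camera it possesses.
; On possession it caches the pawn if it is a BP_SecurityCamera.
; Perception updates from actors without the "AI" tag are filtered by sense class display name, with only sight handled.
; HandleSight prints seen/lost debug text, then forwards the result and target to the cached camera if valid.
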(event `self.AIPerception.OnTargetPerceptionUpdated`
  (params (Actor :type "Actor Object Reference") (Stimulus :type "AIStimulus Structure"))
  (if (not (`self.ActorHasTag` Actor "AI"))
    (bind _returnvalue (`AIPerceptionSystem.GetSenseClassForStimulus` Stimulus))
    (switch `string` (`KismetSystemLibrary.GetClassDisplayName` _returnvalue)
      (:`AISense_Sight`
        (`self.Handle Sight` (`.bSuccessfullySensed` (break `AIStimulus` Stimulus)) Actor)))))

(event `self.ReceivePossess`
  (params (PossessedPawn :type "Pawn Object Reference"))
  (bind _asbp_security_camera (cast `/Game/Blueprints/AI/BP_SecurityCamera` PossessedPawn))
  (set `self.As BP Security Camera` _asbp_security_camera))

(fn `Handle Sight`
  (params (`Successfully Sensed` :type Boolean) (Target :type "Actor Object Reference"))
  (if `Successfully Sensed`
    (`KismetSystemLibrary.PrintText` "I see the player now")
    (else
      (`KismetSystemLibrary.PrintText` "I don't see the player now" true true (struct :`R` 1.0 :`G` 0.176429 :`B` 0.158284 :`A` 1.0))))
  (bind _as_bp_security_camera (`self.As BP Security Camera`)
    (:`then`
      (`/Game/Blueprints/AI/BP_SecurityCamera.HandleSight` _as_bp_security_camera `Successfully Sensed` Target))
    (:`else`)))

(fn `UserConstructionScript`)