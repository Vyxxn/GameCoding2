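; BP_NextLevel is a level-transition trigger that saves the player's items before loading another level.
; When BP_FirstPersonCharacter overlaps it, it passes the character's belt and backpack inventory contents to GM_SaveLoad's Save function.
; It then opens the level held in its Level object reference.
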(event `self.ReceiveActorBeginOverlap`
  (params (OtherActor :type "Actor Object Reference"))
  (bind _asbp_first_person_character (cast `/Game/FirstPerson/Blueprints/BP_FirstPersonCharacter` OtherActor))
  (bind _asgm_save_load (cast `/Game/Blueprints/SavingAndLoading/GM_SaveLoad` (`GameplayStatics.GetGameMode`)))
  (`/Game/Blueprints/SavingAndLoading/GM_SaveLoad.Save` :`self` _asgm_save_load :`Belt` (`/Game/Blueprints/BPC_Inventory.EnumInv` (`/Game/FirstPerson/Blueprints/BP_FirstPersonCharacter.BPC_InvBelt` _asbp_first_person_character)) :`Inventory` (`/Game/Blueprints/BPC_Inventory.EnumInv` (`/Game/FirstPerson/Blueprints/BP_FirstPersonCharacter.BPC_InvBackpack` _asbp_first_person_character)))
  (`GameplayStatics.OpenLevelBySoftObjectPtr` (`self.Level`)))

(fn `UserConstructionScript`)