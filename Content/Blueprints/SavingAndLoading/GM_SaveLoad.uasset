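; Game mode that saves and loads the player and per-level state, loading both on BeginPlay.
; Player data (belt, backpack, last transform) lives in an SG_Player slot, applied to the first-person character's inventory components, capsule and control rotation; a zero saved location skips repositioning.
; Level state uses a separate SG_LevelState slot named from SlotName plus the level name, which restores actor state on load.
; Save writes both slots.
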(event `self.ReceiveBeginPlay`
  (`KismetSystemLibrary.PrintText` "GM_SaveLoad is running")
  (`self.Load Player`))

(event `Load Player`
  (bind _last_position (`/Game/Blueprints/SavingAndLoading/SG_Player.Last Position` (`self.PlayerSave`)))
  (`|ExecutionSequence`
    (:`then_0`
      ; File Management
      (bind _returnvalue (`GameplayStatics.DoesSaveGameExist` (`self.Slot Name`)))
      (if _returnvalue
        (bind _returnvalue_2 (`GameplayStatics.LoadGameFromSlot` (`self.Slot Name`)))
        (bind _assg_player (cast `/Game/Blueprints/SavingAndLoading/SG_Player` _returnvalue_2))
        (set `self.PlayerSave` _assg_player) ; We have linked the game mode's playerSave with the "save-to-file" player save
        (bind _asbp_first_person_character (cast `/Game/FirstPerson/Blueprints/BP_FirstPersonCharacter` (`GameplayStatics.GetPlayerCharacter` 0)))
        (`/Game/Blueprints/BPC_Inventory.SetInventory` (`/Game/FirstPerson/Blueprints/BP_FirstPersonCharacter.BPC_InvBelt` _asbp_first_person_character) (`/Game/Blueprints/SavingAndLoading/SG_Player.Belt` (`self.PlayerSave`)))
        (`/Game/Blueprints/BPC_Inventory.SetInventory` (`/Game/FirstPerson/Blueprints/BP_FirstPersonCharacter.BPC_InvBackpack` _asbp_first_person_character) (`/Game/Blueprints/SavingAndLoading/SG_Player.Inventory` (`self.PlayerSave`)))
        ; is there save data for the location
        (if (not (`KismetMathLibrary.EqualExactly_VectorVector` (.location _last_position)))
          (`SceneComponent.K2_SetWorldTransform` (`Character.CapsuleComponent` _asbp_first_person_character) _last_position false false)
          ; load player rotation
          (`Controller.SetControlRotation` (`GameplayStatics.GetPlayerController` 0) (.rotation _last_position)))
        (else
          (bind _returnvalue_3 (`GameplayStatics.CreateSaveGameObject` "/Game/Blueprints/SavingAndLoading/SG_Player.SG_Player_C"))
          (set `self.PlayerSave` _returnvalue_3))))
    (:`then_1`
      (`self.LoadLevel`))))

(event `Save`
  (params (Belt :type "Array of /Game/Blueprints/E_Item Enum") (Inventory :type "Array of /Game/Blueprints/E_Item Enum") (`Last Position` :type "Transform Structure"))
  (bind _playersave (`self.PlayerSave`))
  (`|ExecutionSequence`
    (:`then_0`
      (set `/Game/Blueprints/SavingAndLoading/SG_Player.Belt` Belt _playersave)
      (set `/Game/Blueprints/SavingAndLoading/SG_Player.Inventory` Inventory _playersave)
      (set `/Game/Blueprints/SavingAndLoading/SG_Player.Last Position` `Last Position` _playersave)
      (bind _returnvalue (`GameplayStatics.SaveGameToSlot` (`self.PlayerSave`) (`self.Slot Name`)))
      (if _returnvalue
        (`KismetSystemLibrary.PrintText` "Game saved to slot")
        (else
          (`KismetSystemLibrary.PrintText` "Could not save game to slot"))))
    (:`then_1`
      (`self.SaveLevel`))))

(event `LoadLevel`
  (bind _returnvalue (`GameplayStatics.GetCurrentLevelName` true))
  (bind _returnvalue_2 (`KismetStringLibrary.Concat_StrStr` (`self.Slot Name`) "_" _returnvalue))
  (bind _returnvalue_3 (`GameplayStatics.DoesSaveGameExist` _returnvalue_2))
  (if _returnvalue_3
    (bind _returnvalue_4 (`GameplayStatics.LoadGameFromSlot` _returnvalue_2))
    (bind _assg_level_state (cast `/Game/Blueprints/SavingAndLoading/SG_LevelState` _returnvalue_4))
    (bind _output_get (set `self.Level State` _assg_level_state))
    (`/Game/Blueprints/SavingAndLoading/SG_LevelState.Load Actor State` _output_get)
    (else
      (bind _returnvalue_5 (`GameplayStatics.CreateSaveGameObject` "/Game/Blueprints/SavingAndLoading/SG_LevelState.SG_LevelState_C"))
      (set `self.Level State` _returnvalue_5))))

(event `SaveLevel`
  (bind _returnvalue (`GameplayStatics.GetCurrentLevelName` true))
  (`GameplayStatics.SaveGameToSlot` (`self.Level State`) (`KismetStringLibrary.Concat_StrStr` (`self.Slot Name`) "_" _returnvalue)))

(fn `UserConstructionScript`)