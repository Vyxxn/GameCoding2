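; BP_Grenade is a prototype grenade item that can be picked up, dropped and used.
; Pickup disables the sphere's collision and returns its item type, while Drop restores collision and physics and launches it forward with an impulse.
; Use line-traces forward and prints "Kaboom" on a hit, but its radial damage node is unconnected.
; AltUse draws a debug line to GetClosest's result, though that function is an empty stub.
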(event `/Game/Blueprints/BPI_Item.Drop`
  (bind _sphere (`self.Sphere`))
  (`PrimitiveComponent.SetCollisionEnabled` (`self.Sphere`) "QueryAndPhysics")
  (`PrimitiveComponent.SetSimulatePhysics` _sphere true)
  (`PrimitiveComponent.AddImpulse` _sphere (* (`SceneComponent.GetForwardVector` (`self.Sphere`)) 1000.0) "None" true))

(event `/Game/Blueprints/BPI_Item.Use`
  (bind _returnvalue (`SceneComponent.K2_GetComponentLocation` (`self.Sphere`)))
  (bind (_outhit _returnvalue_2) (`KismetSystemLibrary.LineTraceSingle` :`Start` _returnvalue :`End` (+ _returnvalue (* (`SceneComponent.GetForwardVector` (`self.Sphere`)) 400.0)) :`TraceChannel` "TraceTypeQuery1" :`DrawDebugType` "ForDuration"))
  (if _returnvalue_2
    (`KismetSystemLibrary.PrintText` "Kaboom")))

(event `/Game/Blueprints/BPI_Item.AltUse`
  (bind _closestactor (`self.GetClosest` _))
  (`KismetSystemLibrary.DrawDebugLine` (`self.K2_GetActorLocation`) (`self.K2_GetActorLocation` _closestactor) (struct :`R` 1.0 :`G` 0.161384 :`B` 0.634166 :`A` 1.0) 4.0 5.0))

(fn `GetClosest`
  (params (ArrayOfActors :type "Array of Actor Object Reference (by ref)") (Origin :type "Actor Object Reference"))
  (returns (ClosestACtor :type "Actor Object Reference"))
  (return null))

(fn `Pickup`
  (params (Owner :type "/Game/Blueprints/BPC_Interact Object Reference"))
  (returns (`Item Type` :type "/Game/Blueprints/E_Item Enum"))
  (`PrimitiveComponent.SetCollisionEnabled` (`self.Sphere`) "NoCollision") ; Stop the grenade from pushing the player off the map
  (return (`self.Item Type`)))

(fn `UserConstructionScript`)