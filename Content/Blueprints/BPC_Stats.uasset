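; Player stats component that tracks health, stamina and experience, and creates the W_PlayerStats widget to show them as bars.
; Each stat is packed into a vector: health holds min, max and current, while experience holds level, next threshold and current XP.
; ChangeHealth reloads the level on death, and ChangeXP handles level-ups with a growing threshold.
; SetXP is an empty stub, and ChangeXP's bar update has unconnected zero inputs.
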(event `self.ReceiveBeginPlay`
  (bind _statswidget (`self.StatsWidget`))
  (bind (_health_x _health_y _health_z) (`KismetMathLibrary.BreakVector` (`self.Health`)))
  (bind (_stamina_x _stamina_y _stamina_z) (`KismetMathLibrary.BreakVector` (`self.Stamina`)))
  (bind (_experience_x _experience_y _experience_z) (`KismetMathLibrary.BreakVector` (`self.Experience`)))
  (`|ExecutionSequence`
    (:`then_0`
      (bind _returnvalue (`|CreateWidget` "/Game/UI/W_PlayerStats.W_PlayerStats_C"))
      (bind _output_get (set `self.StatsWidget` _returnvalue))
      (`UserWidget.AddToViewport` _output_get 0))
    (:`then_1`
      (`self.SetHealth` _health_x _health_y _health_z)
      (`ProgressBar.SetPercent` (`/Game/UI/W_PlayerStats.StaminaBar` _statswidget) _stamina_z)
      (`ProgressBar.SetPercent` (`/Game/UI/W_PlayerStats.XPBar` _statswidget) _experience_z))))

(fn `ChangeHealth`
  (params (`By Amount` :type "Float (double-precision)"))
  (bind (_health_x _health_y _health_z) (`KismetMathLibrary.BreakVector` (`self.Health`)))
  (bind (_health_x_2 _health_y_2 _health_z_2) (`KismetMathLibrary.BreakVector` (`self.Health`)))
  (bind _returnvalue (+ _health_z `By Amount`))
  (set `self.Health` (`KismetMathLibrary.MakeVector` _health_x _health_y _returnvalue))
  (`ProgressBar.SetPercent` (`/Game/UI/W_PlayerStats.HealthBar` (`self.StatsWidget`)) (/ _health_z_2 (- _health_y_2 _health_x_2))) ; 0-100 is easy, just return health.z\nWhat if 25-150?
  (if (<= _returnvalue 0.0)
    (`KismetSystemLibrary.PrintText` "Player has died")
    (bind _returnvalue_2 (`GameplayStatics.GetCurrentLevelName` true))
    (`GameplayStatics.OpenLevel` (`KismetStringLibrary.Conv_StringToName` _returnvalue_2))))

(fn `ChangeXP`
  (params (`By Amount` :type "Float (double-precision)"))
  (bind (_experience_x _experience_y _experience_z) (`KismetMathLibrary.BreakVector` (`self.Experience`)))
  (bind (_experience_x_2 _experience_y_2 _experience_z_2) (`KismetMathLibrary.BreakVector` (`self.Experience`)))
  (bind (_experience_x_3 _experience_y_3) (`KismetMathLibrary.BreakVector` (`self.Experience`)))
  (bind _returnvalue (+ _experience_z_2 `By Amount`))
  (set `self.Experience` (`KismetMathLibrary.MakeVector` _experience_x_2 _experience_y_2 _returnvalue))
  (`ProgressBar.SetPercent` (`/Game/UI/W_PlayerStats.XPBar` (`self.StatsWidget`)) (/ 0.0 (- 0.0 0.0))) ; 0-100 is easy, just return health.z\nWhat if 25-150?
  (if (>= _returnvalue _experience_y_3)
    (set `self.Experience` (`KismetMathLibrary.MakeVector` (+ _experience_x 1.0) (* _experience_y 1.5) (* _experience_z 0.0)))))

(fn `SetHealth`
  (params (`Health X` :type "Float (double-precision)" :default -1.0) (`Health Y` :type "Float (double-precision)" :default -1.0) (`Health Z` :type "Float (double-precision)" :default -1.0))
  (locals (MinHealth :type "Float (double-precision)") (MaxHealth :type "Float (double-precision)") (CurrentHealth :type "Float (double-precision)"))
  (bind (_health_x _health_y _health_z) (`KismetMathLibrary.BreakVector` (`self.Health`)))
  ; setting temp variables to health's current values
  (set `local.MinHealth` (`local.Health X`))
  (set `local.MaxHealth` (`local.Health Y`))
  (set `local.CurrentHealth` (`local.Health Z`))
  (if (!= `Health X` -1.0)
    (set `local.MinHealth` `Health X`) ; store new min health
  )
  (if true
    (set `local.MaxHealth` `Health Y`))
  (if true
    (set `local.CurrentHealth` `Health Z`))
  (set `self.Health` (`KismetMathLibrary.MakeVector` (`local.MinHealth`) (`local.MaxHealth`) (`local.CurrentHealth`)))
  ; Update the widget code
  (`ProgressBar.SetPercent` (`/Game/UI/W_PlayerStats.HealthBar` (`self.StatsWidget`)) (/ _health_z (- _health_y _health_x))))

(fn `SetXP`
  (params (InputPin :type "Float (double-precision)") (InputPin1 :type "Float (double-precision)"))
  (locals (`Current XP` :type "Float (double-precision)") (`Current Level` :type "Float (double-precision)") (`XP to Next Level` :type "Float (double-precision)")))