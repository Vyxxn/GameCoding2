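; Actor component that stores an inventory as an array of item enums, one per slot.
; GetSlot resolves a slot's enum to its item details through GetItemDetails, which linearly searches DT_Items rows for a matching EnumName.
; SetSlot writes one slot and calls OnSlotUpdated with its index, while SetInventory replaces the whole array and calls OnSetInventory, so listeners can react to changes.
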(fn `GetItemDetails`
  (params (`Requested Item` :type "/Game/Blueprints/E_Item Enum" :default "NewEnumerator0"))
  (returns (`Item Details` :type "/Game/Blueprints/S_Item Structure"))
  (bind _outrownames (`DataTableFunctionLibrary.GetDataTableRowNames` "/Game/Blueprints/DataTables/DT_Items.DT_Items"))
  (for _array_element _outrownames
    (bind _returnvalue (`|GetDataTableRow` "/Game/Blueprints/DataTables/DT_Items.DT_Items" _array_element)
      (:`then`
        (if (`|EnumEquality` (`.EnumName_18_B9CE5B474CD0002CE8C520B1A8A658C6` (break `/Game/Blueprints/S_Item` _returnvalue)) `Requested Item`)
          (return _returnvalue) ; Give an item
        )))))

(fn `GetSlot`
  (params (`Requested Slot` :type Integer))
  (returns (`Item Details` :type "/Game/Blueprints/S_Item Structure"))
  (bind _item_details (`self.GetItemDetails` (`|GetArrayItem` (`self.EnumInv`) `Requested Slot`)))
  (return _item_details))

(fn `SetInventory`
  (params (EnumInv :type "Array of /Game/Blueprints/E_Item Enum"))
  (set `self.EnumInv` EnumInv)
  (`self.OnSetInventory`))

(fn `SetSlot`
  (params (ItemType :type "/Game/Blueprints/E_Item Enum" :default "E_Item_MAX") (Index :type Integer))
  (`KismetArrayLibrary.Array_Set` (`self.EnumInv`) Index ItemType)
  (`self.OnSlotUpdated` Index))