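; BP_Spawner is a spawner actor that calls an empty SpawnThing event shortly after BeginPlay, with no spawn logic of its own.
; When not Looping, its Activate event destroys the actor.
; A first-person character overlapping the Trigger of a non-looping spawner calls AddActor on GM_SaveLoad's LevelState, apparently to record it for save/load.
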(event `self.ReceiveBeginPlay`
  (`KismetSystemLibrary.Delay` 0.2)
  (`self.Spawn Thing`))

(event `Spawn Thing`)

(event `/Game/Blueprints/BPI_Activatable.Activate`
  (if (not (`self.Looping`))
    (`self.K2_DestroyActor`)))

(event `self.Trigger.OnComponentBeginOverlap`
  (params (OverlappedComponent :type "PrimitiveComponent Object Reference") (OtherActor :type "Actor Object Reference") (OtherComp :type "PrimitiveComponent Object Reference") (OtherBodyIndex :type Integer) (bFromSweep :type Boolean) (SweepResult :type "HitResult Structure (by ref)"))
  (if (not (`self.Looping`))
    (cast `/Game/FirstPerson/Blueprints/BP_FirstPersonCharacter` OtherActor)
    (bind _asgm_save_load (cast `/Game/Blueprints/SavingAndLoading/GM_SaveLoad` (`GameplayStatics.GetGameMode`)))
    (`/Game/Blueprints/SavingAndLoading/SG_LevelState.Add Actor` (`/Game/Blueprints/SavingAndLoading/GM_SaveLoad.Level State` _asgm_save_load) null)))

(fn `UserConstructionScript`)