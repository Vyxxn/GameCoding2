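; BP_Blaster is a pickup weapon item with primary and alternate use, still at a prototype stage.
; Pickup disables box collision and returns the item type; Drop restores collision and physics, then launches the box forward.
; Use runs a short forward visibility trace and prints "Pow" on a hit, with point damage left unconnected.
; AltUse draws a debug line toward the GetClosest result, but that function's body is empty.
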(event `/Game/Blueprints/BPI_Item.Drop`
  (bind _box (`self.Box`))
  (`PrimitiveComponent.SetCollisionEnabled` (`self.Box`) "QueryAndPhysics")
  (`PrimitiveComponent.SetSimulatePhysics` _box true)
  (`PrimitiveComponent.AddImpulse` _box (* (`SceneComponent.GetForwardVector` _box) 1000.0) "None" true))

(event `/Game/Blueprints/BPI_Item.Use`
  (bind _box (`self.Box`))
  (bind _returnvalue (`SceneComponent.K2_GetComponentLocation` _box))
  (bind (_outhit _returnvalue_2) (`KismetSystemLibrary.LineTraceSingle` :`Start` _returnvalue :`End` (+ _returnvalue (* (`SceneComponent.GetForwardVector` _box) 400.0)) :`TraceChannel` "TraceTypeQuery1" :`DrawDebugType` "ForDuration"))
  (if _returnvalue_2
    (`KismetSystemLibrary.PrintText` "Pow")))

(event `/Game/Blueprints/BPI_Item.AltUse`
  (bind _closestactor (`self.GetClosest` :`Origin` self))
  (`KismetSystemLibrary.DrawDebugLine` (`self.K2_GetActorLocation`) (`self.K2_GetActorLocation` _closestactor) (struct :`R` 1.0 :`G` 0.161384 :`B` 0.634166 :`A` 1.0) 4.0 5.0))

(fn `GetClosest`
  (params (ArrayOfActors :type "Array of Actor Object Reference (by ref)") (Origin :type "Actor Object Reference"))
  (returns (ClosestACtor :type "Actor Object Reference"))
  (return null))

(fn `Pickup`
  (params (Owner :type "/Game/Blueprints/BPC_Interact Object Reference"))
  (returns (`Item Type` :type "/Game/Blueprints/E_Item Enum"))
  (`PrimitiveComponent.SetCollisionEnabled` (`self.Box`) "NoCollision") ; Stop the key from pushing the player off the map
  (return (`self.Item Type`)))

(fn `UserConstructionScript`)